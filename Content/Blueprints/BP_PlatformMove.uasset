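; BP_PlatformMove is an actor that slides platforms back and forth along world Y by Distance, starting at BeginPlay.
; It caches each platform's start location, then two timelines, Movement and ReverseMovement, restart each other endlessly at a rate set by Time.
; Both timelines are driven inside the ForEach loop, so their updates see only the last platform.
; The construction script destroys the Sphere component.
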(event Custom|PlayMovement
  (bind _platforms (Variables|Default|GetPlatforms))
  (if (Utilities|Array|IsNotEmpty _platforms)
    (Components|Timeline|SetPlayRate (Variables|Default|GetReverseMovement) (/ 1.0 (Variables|Default|GetTime)))
    (for (_array_element _array_index) _platforms
      (Utilities|Array|SetArrayElem (Variables|Default|GetNewVar) _array_index (Transformation|GetActorLocation _array_element) true)
      (bind _newtrack_0 (Timeline|Movement PlayFromStart)
        (:Update
          (Transformation|SetActorLocation _array_element (Math|Vector|Lerp(Vector) (Utilities|Array|Get(acopy) (Variables|Default|GetNewVar) _array_index) (+ (Utilities|Array|Get(acopy) (Variables|Default|GetNewVar) _array_index) (Math|Vector|MakeVector 0.0 (* (Variables|Default|GetDistance) _newtrack_0) 0.0)) _newtrack_0) false true))
        (:Finished
          (bind _newtrack_0_2 (Timeline|ReverseMovement PlayFromStart)
            (:Update
              (Transformation|SetActorLocation _array_element (Math|Vector|Lerp(Vector) (+ (Utilities|Array|Get(acopy) (Variables|Default|GetNewVar) _array_index) (Math|Vector|MakeVector 0.0 (* (Variables|Default|GetDistance) _newtrack_0) 0.0)) (Utilities|Array|Get(acopy) (Variables|Default|GetNewVar) _array_index) _newtrack_0_2) false true))
            (:Finished
              (Timeline|Movement PlayFromStart))))))))

(event EventBeginPlay
  (CallFunction|PlayMovement))

(event Collision|EventActorBeginOverlap
  (params (OtherActor :type Actor%20Object%20Reference)))

(event EventTick
  (params (DeltaSeconds :type Float%20%28single-precision%29)))

(fn ConstructionScript
  (Components|DestroyComponent (Variables|Default|GetSphere)))